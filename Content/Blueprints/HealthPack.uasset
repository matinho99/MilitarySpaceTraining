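; HealthPack is a pickup actor that heals a player SpaceSoldierCharacter or an EnemySoldier whose HP is below max.
; On box overlap it matches the actor's exact class, plays a heal sound at that actor and calls its UseHealthPack.
; Both branches share a cooldown that disables and hides the pack, then restores it after a delay.
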(event `self.Box.OnComponentBeginOverlap`
  (params (OverlappedComponent :type "PrimitiveComponent Object Reference") (OtherActor :type "Actor Object Reference") (OtherComp :type "PrimitiveComponent Object Reference") (OtherBodyIndex :type Integer) (bFromSweep :type Boolean) (SweepResult :type "HitResult Structure (by ref)"))
  (bind _returnvalue (`GameplayStatics.GetObjectClass` OtherActor))
  (if (not (`self.Disabled`))
    (`|ExecutionSequence`
      (:`then_0`
        (if (== _returnvalue "/Game/Character/SpaceSoldierCharacter.SpaceSoldierCharacter_C")
          (bind _asspace_soldier_character (cast `/Game/Character/SpaceSoldierCharacter` OtherActor))
          (if (< (`/Game/Character/SpaceSoldierCharacter.HP` _asspace_soldier_character) (`/Game/Character/SpaceSoldierCharacter.MaxHP` _asspace_soldier_character))
            (`GameplayStatics.PlaySoundAtLocation` "/Game/Audio/HealSFX.HealSFX" (`self.K2_GetActorLocation` _asspace_soldier_character) (struct) 1.0 1.0 0.0 null null null)
            (`/Game/Character/SpaceSoldierCharacter.UseHealthPack` _asspace_soldier_character)
            (set `self.Disabled` true :!label _label)
            (`self.SetActorHiddenInGame` true)
            (`KismetSystemLibrary.Delay` (`self.Cooldown`))
            (`self.SetActorHiddenInGame` false)
            (set `self.Disabled` false))))
      (:`then_1`
        (if (== _returnvalue "/Game/AI/EnemySoldier.EnemySoldier_C")
          (bind _asenemy_soldier (cast `/Game/AI/EnemySoldier` OtherActor))
          (if (< (`/Game/AI/EnemySoldier.HP` _asenemy_soldier) (`/Game/AI/EnemySoldier.MaxHP` _asenemy_soldier))
            (`GameplayStatics.PlaySoundAtLocation` "/Game/Audio/HealSFX.HealSFX" (`self.K2_GetActorLocation` _asenemy_soldier) (struct) 1.0 1.0 0.0 null null null)
            (`/Game/AI/EnemySoldier.UseHealthPack` _asenemy_soldier)
            (goto _label)))))))

(fn `UserConstructionScript`)