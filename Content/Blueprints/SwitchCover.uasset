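; SwitchCover is a Blueprint that moves a Cover component vertically while a Pawn is inside its Box volume.
; Each tick it polls the Box for overlapping Pawns, playing CoverTimeline when any are present and reversing it otherwise.
; The timeline track scales the Box's relative Z to set the Cover's relative height, with X and Y held at zero.
; BeginPlay sets the timeline's play rate from Speed.
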(event `self.ReceiveBeginPlay`
  (`TimelineComponent.SetPlayRate` (`self.CoverTimeline`) (`self.Speed`)))

(event `self.ReceiveTick`
  (params (DeltaSeconds :type "Float (single-precision)"))
  (if (> (`KismetArrayLibrary.Array_Length` (`PrimitiveComponent.GetOverlappingActors` (`self.Box`) "/Script/Engine.Pawn")) 0)
    (bind (_direction _track_0) (`Timeline|CoverTimeline` :!label _label)
      (:`Update`
        (`SceneComponent.K2_SetRelativeLocation` (`self.Cover`) (`KismetMathLibrary.MakeVector` 0.0 0.0 (* (.z (`SceneComponent.RelativeLocation` (`self.Box`))) _track_0)) false false)))
    (else
      (goto _label :!via `Reverse`))))

(fn `UserConstructionScript`)